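; BP_NPC_Character is an NPC that wanders the level on its own from BeginPlay, using AI navigation.
; MoveNPCS picks a random actor from its Targets array, or a random navigable point within a radius of itself when that array is empty.
; AIMoveTo then moves it there, and the event calls itself again after a pause on success or a shorter one on failure, looping indefinitely.
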(event `self.ReceiveBeginPlay`
  (`self.MoveNPCS`))

(event `MoveNPCS`
  ; Test Targets
  (if (`KismetArrayLibrary.Array_IsEmpty` (`self.Targets`))
    ; Get Random Position
    (bind _randomlocation (`NavigationSystemV1.K2_GetRandomLocationInNavigableRadius` (`self.K2_GetActorLocation` self) 1000.0 null null))
    (set `self.Random Location` _randomlocation)
    (else
      ; Get Random Targets
      (set `self.Random Location` (`self.K2_GetActorLocation` (`KismetArrayLibrary.Array_Random` (`self.Targets`))))))
  ; Move Pawn to position
  (`|AIMoveTo` self (`self.Random Location`) null
    (:`OnSuccess`
      (`KismetSystemLibrary.Delay` 2.0))
    (:`OnFail`
      (`KismetSystemLibrary.Delay` 0.1)))
  (`self.MoveNPCS`))

(fn `UserConstructionScript`)