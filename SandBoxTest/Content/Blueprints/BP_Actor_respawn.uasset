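; Respawn actor that teleports one child actor (TargetToRespawn) to the transform of another (RespawnTarget).
; On BeginPlay it binds to the RequestRespawn event on BP_GameInstance, which triggers the teleport without sweeping and prints a debug message.
; A second handler, RespawnActor_Event, leads to the same teleport, but its binding node is never executed.
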(event `RespawnActor_Event`
  ; Bind event
  (`KismetSystemLibrary.PrintText` "Respawn Component" true true (struct :`R` 0.004155 :`G` 1.0 :`A` 1.0))
  ; Respawn child actor
  (`self.K2_SetActorTransform` (`ChildActorComponent.ChildActor` (`self.Target_to_respawn`)) (`self.GetTransform` (`ChildActorComponent.ChildActor` (`self.Respawn_Target`))) false true :!label _label))

(event `self.ReceiveBeginPlay`
  ; Bind to external event
  (bind _asbp_game_instance (cast `/Game/Blueprints/BP_GameInstance` (`GameplayStatics.GetGameInstance`)))
  (add `/Game/Blueprints/BP_GameInstance.RequestRespawn` _asbp_game_instance (delegate `OnResquestRespawn`)))

(event `OnResquestRespawn`
  ; Bind to external event
  (`KismetSystemLibrary.PrintText` "On RequestRespawn" true true (struct :`R` 1.0 :`B` 0.69501 :`A` 1.0))
  (goto _label))

(fn `UserConstructionScript`)