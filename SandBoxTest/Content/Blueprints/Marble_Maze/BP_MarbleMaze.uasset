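; Marble maze Blueprint that tilts its MazeBoard component in response to player input.
; Enhanced Input actions for pitch and roll each add a local rotation scaled by RotationSpeed.
; Each then rewrites the relative rotation, clamping its own axis to a limited tilt range and zeroing yaw to stop drift.
; The pitch handler also prints its input value to screen.
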(event `EnhancedInput|/Game/Inputs/Marble_Maze/IA_Pitch`
  (params (ActionValue :type "Float (double-precision)") (ElapsedSeconds :type "Float (double-precision)") (TriggeredSeconds :type "Float (double-precision)") (InputAction :type "InputAction Object Reference" :default "/Game/Inputs/Marble_Maze/IA_Pitch.IA_Pitch"))
  (bind _maze_board (`self.Maze_Board`))
  (bind (_relativerotation_roll _relativerotation_pitch) (`KismetMathLibrary.BreakRotator` (`SceneComponent.RelativeRotation` _maze_board)))
  (:`Triggered`
    (`KismetSystemLibrary.PrintString` (`KismetStringLibrary.Conv_DoubleToString` ActionValue) true true (struct :`G` 0.66 :`B` 1.0 :`A` 1.0) 2.0 "Pitch")
    (`SceneComponent.K2_AddLocalRotation` (`self.Maze_Board`) (`KismetMathLibrary.MakeRotator` 0.0 (* ActionValue (`self.RotationSpeed`))) false false)
    (`SceneComponent.K2_SetRelativeRotation` _maze_board (`KismetMathLibrary.MakeRotator` _relativerotation_roll (`KismetMathLibrary.ClampAngle` _relativerotation_pitch -15.0 15.0)) false false)))

(event `EnhancedInput|/Game/Inputs/Marble_Maze/IA_Roll`
  (params (ActionValue :type "Float (double-precision)") (ElapsedSeconds :type "Float (double-precision)") (TriggeredSeconds :type "Float (double-precision)") (InputAction :type "InputAction Object Reference" :default "/Game/Inputs/Marble_Maze/IA_Roll.IA_Roll"))
  (bind _maze_board (`self.Maze_Board`))
  (bind (_relativerotation_roll _relativerotation_pitch) (`KismetMathLibrary.BreakRotator` (`SceneComponent.RelativeRotation` _maze_board)))
  (:`Triggered`
    (`SceneComponent.K2_AddLocalRotation` (`self.Maze_Board`) (`KismetMathLibrary.MakeRotator` (* ActionValue (`self.RotationSpeed`))) false false)
    (`SceneComponent.K2_SetRelativeRotation` _maze_board (`KismetMathLibrary.MakeRotator` (`KismetMathLibrary.ClampAngle` _relativerotation_roll -15.0 15.0) _relativerotation_pitch) false false)))

(fn `UserConstructionScript`)