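; BP_Maze_Ball is the player ball for a marble maze, handling respawn when it falls out of the level.
; It saves its spawn location on BeginPlay and checks its height every Tick.
; When the height drops to RespawnLimit or below, it teleports back to the saved start position and prints the Z value for debugging.
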(event `self.ReceiveBeginPlay`
  ; Save Start Position
  (set `self.StartPosition` (`self.K2_GetActorLocation`)))

(event `self.ReceiveTick`
  (params (DeltaSeconds :type "Float (single-precision)"))
  (bind _z (.z (`self.K2_GetActorLocation`)))
  ; Test ball position to respawn
  (if (<= _z (`self.RespawnLimit`))
    (`self.ResetPosition`)
    ; Debug Z position
    (`KismetSystemLibrary.PrintText` (`KismetTextLibrary.Conv_DoubleToText` _z "HalfToEven") true true (struct :`G` 0.66 :`B` 1.0 :`A` 1.0) 2.0 "ball position")))

(fn `ResetPosition`
  (`self.K2_SetActorLocation` (`self.StartPosition`) false true))

(fn `UserConstructionScript`)